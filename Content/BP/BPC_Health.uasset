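; BPC_Health is a health component that tracks hit points and death for its owner.
; BeginPlay stores the starting HP as MaxHP and binds a debug "DEATH" print to its OnDeath dispatcher.
; HandleDmg subtracts damage, clamps HP to a fixed 0–100 range rather than MaxHP, and at zero sets IsDead and calls OnDeath.
; No guard checks IsDead, so further hits at zero HP fire OnDeath again.
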(event `self.ReceiveBeginPlay`
  (set `self.MaxHP` (`self.HP`))
  (add `self.OnDeath` (delegate `CustomEvent`)))

(event `CustomEvent`
  (`KismetSystemLibrary.PrintString` "DEATH"))

(event `HandleDmg`
  (params (NewParam :type "Float (double-precision)"))
  (bind _output_get (set `self.HP` (`KismetMathLibrary.FClamp` (- (`self.HP`) NewParam) 0.0 100.0)))
  (if (<= _output_get 0.0)
    (set `self.IsDead` true)
    (`self.OnDeath`)))